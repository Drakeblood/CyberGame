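; CyberGame game mode that sets up the current mission and delivers its startup emails at BeginPlay.
; If its own mission name is empty, it writes a default row from the protector missions DataTable into the game instance.
; It then copies the game instance's mission and, after a short delay, passes each startup mail to SendEmail.
; SendEmail adds the mail to the monitor's mail app and shows a Polish new-mail HUD notification.
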(event EventBeginPlay
  (if (Utilities|Enum|Equal(Enum) (.name (Variables|Default|GetCurrentMission)) (Utilities|Text|MakeLiteralText ""))
    (Utilities|FlowControl|Sequence
      (:then_0
        (bind _returnvalue (Utilities|GetDataTableRow "/Game/_CyberGame/Missions/DT_ProtectorMissions.DT_ProtectorMissions" "NewRow")
          (:then
            (Variables|/Game/_CyberGame/Blueprints/System/GI_CyberGame.GI_CyberGame_C|SetCurrentMission (CallFunction|GetCyberGameInstance) _returnvalue))))
      (:then_1
        (Variables|Default|SetCurrentMission (Variables|/Game/_CyberGame/Blueprints/System/GI_CyberGame.GI_CyberGame_C|GetCurrentMission (CallFunction|GetCyberGameInstance)) :!label _label)
        (Utilities|FlowControl|Delay 2.0)
        (for _array_element (.startupmails (Variables|Default|GetCurrentMission))
          (CallFunction|SendEmail _array_element))))
    (else
      (goto _label))))

(fn ConstructionScript)

(fn SendEmail
  (params (DataTableRowHandle :type Data%20Table%20Row%20Handle%20Structure%20%28by%20ref%29))
  (Default|AddMail (Variables|/Game/_CyberGame/Blueprints/Widget/WBP_Monitor.WBP_Monitor_C|GetWBP_MailApp (Variables|Default|GetWBP_Monitor)) DataTableRowHandle)
  (Default|AddNotification (Variables|Default|GetWBP_HUD) "Nowy mail!"))