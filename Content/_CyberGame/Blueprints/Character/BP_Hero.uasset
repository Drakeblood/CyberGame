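; BP_Hero is the player character, handling movement, look, world interaction and widget clicks through Enhanced Input.
; Each tick, a line trace from the eye viewpoint finds InteractableInterface actors, focuses those that allow interaction and shows their prompt on the PC_CyberGame hero widget.
; Interacting messages the focused actor, then clears focus and hides the prompt.
; IA_LPM forwards left mouse presses and releases to a WidgetInteraction component.
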(event Input|EnhancedActionEvents|EnhancedInputActionIA_Move
  (params (ActionValue :type Vector%202D%20Structure) (ElapsedSeconds :type Float%20%28double-precision%29) (TriggeredSeconds :type Float%20%28double-precision%29) (InputAction :type Input%20Action%20Object%20Reference :default "/Game/_CyberGame/Input/Actions/IA_Move.IA_Move"))
  (Class|CGHeroCharacter|Move (Class|EnhancedInputLibrary|MakeInputActionValueOfType (.x ActionValue) (.y ActionValue) 0.0 "Axis2D")))

(event Input|EnhancedActionEvents|EnhancedInputActionIA_Look
  (params (ActionValue :type Vector%202D%20Structure) (ElapsedSeconds :type Float%20%28double-precision%29) (TriggeredSeconds :type Float%20%28double-precision%29) (InputAction :type Input%20Action%20Object%20Reference :default "/Game/_CyberGame/Input/Actions/IA_Look.IA_Look"))
  (Class|CGHeroCharacter|Look (Class|EnhancedInputLibrary|MakeInputActionValueOfType (.x ActionValue) (.y ActionValue) 0.0 "Axis2D")))

(event Input|EnhancedActionEvents|EnhancedInputActionIA_Interact
  (params (ActionValue :type Boolean) (ElapsedSeconds :type Float%20%28double-precision%29) (TriggeredSeconds :type Float%20%28double-precision%29) (InputAction :type Input%20Action%20Object%20Reference :default "/Game/_CyberGame/Input/Actions/IA_Interact.IA_Interact"))
  (:Started
    (bind _currentinteractable (Variables|Default|GetCurrentInteractable)
      (:then
        (Class|InteractableInterface|Interact(Message) _currentinteractable self)
        (Class|InteractableInterface|Defocus(Message) _currentinteractable self)
        (Variables|Default|SetCurrentInteractable 0)
        (Default|HideInteractionMessage (Variables|/Game/_CyberGame/Blueprints/Player/PC_CyberGame.PC_CyberGame_C|GetWBPHero (Variables|Default|GetPCCyberGame))))
      (:else))))

(event Input|EnhancedActionEvents|EnhancedInputActionIA_LPM
  (params (ActionValue :type Boolean) (ElapsedSeconds :type Float%20%28double-precision%29) (TriggeredSeconds :type Float%20%28double-precision%29) (InputAction :type Input%20Action%20Object%20Reference :default "/Game/_CyberGame/Input/Actions/IA_LPM.IA_LPM"))
  (bind _widgetinteraction (Variables|Default|GetWidgetInteraction))
  (:Started
    (Class|WidgetInteractionComponent|PressPointerKey _widgetinteraction "LeftMouseButton"))
  (:Completed
    (Class|WidgetInteractionComponent|ReleasePointerKey _widgetinteraction "LeftMouseButton")))

(event EventTick
  (params (DeltaSeconds :type Float%20%28single-precision%29))
  (bind (_outlocation _outrotation) (Actor|GetActorEyesViewPoint))
  (bind (_outhit _returnvalue) (Collision|LineTraceByChannel _outlocation (+ _outlocation (* (Math|Vector|GetForwardVector _outrotation) (Variables|Default|GetLineTraceLength))) "TraceTypeQuery3" false 0 "None" true "(R=1.000000,G=0.000000,B=0.000000,A=1.000000)" "(R=0.000000,G=1.000000,B=0.000000,A=1.000000)" 0.1))
  (if (and (Utilities|DoesObjectImplementInterface (.hitactor _outhit) "/Script/CyberGame.InteractableInterface") _returnvalue)
    (if (!= (Variables|Default|GetCurrentInteractable) (.hitactor _outhit))
      (bind _returnvalue_2 (Class|InteractableInterface|CanInteract(Message) (.hitactor _outhit) self))
      (if _returnvalue_2
        (bind _currentinteractable (Variables|Default|GetCurrentInteractable)
          (:then
            (Class|InteractableInterface|Defocus(Message) _currentinteractable self))
          (:else
            _))
        (bind _output_get (Variables|Default|SetCurrentInteractable (.hitactor _outhit)))
        (Class|InteractableInterface|Focus(Message) _output_get self)
        (bind _returnvalue_3 (Class|InteractableInterface|GetInteractionMessage(Message) (Variables|Default|GetCurrentInteractable) self))
        (Default|ShowInteractionMessage (Variables|/Game/_CyberGame/Blueprints/Player/PC_CyberGame.PC_CyberGame_C|GetWBPHero (Variables|Default|GetPCCyberGame)) _returnvalue_3)
        (else
          (bind _currentinteractable_2 (Variables|Default|GetCurrentInteractable :!label _label)
            (:then
              (Class|InteractableInterface|Defocus(Message) _currentinteractable_2 self)
              (Variables|Default|SetCurrentInteractable 0)
              (Default|HideInteractionMessage (Variables|/Game/_CyberGame/Blueprints/Player/PC_CyberGame.PC_CyberGame_C|GetWBPHero (Variables|Default|GetPCCyberGame))))
            (:else)))))
    (else
      (goto _label))))

(event EventBeginPlay)

(event EventPossessed
  (params (NewController :type Controller%20Object%20Reference))
  (Variables|Default|SetPCCyberGame (.AsPC%20Cyber%20Game (Utilities|Casting|CastToPC_CyberGame NewController))))

(fn ConstructionScript)